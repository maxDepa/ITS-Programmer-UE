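; BP_Info is a data model that holds display information for an item or entity: a name, a description and an icon.
; Initialize copies the three fields from a passed Info value into its own variables.
; Separate getter functions expose each field, with no other logic.
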(fn `GetDescription`
  (returns (Description :type String))
  (return (`self.Description`)))

(fn `GetIcon`
  (returns (Icon :type "Texture2D Object Reference"))
  (return (`self.Icon`)))

(fn `GetName`
  (returns (Name :type String))
  (return (`self.Name`)))

(fn `Initialize`
  (params (Info :type "/Game/LOGIC/DTO/ST_Info Structure"))
  (bind (_name _description _icon) (break `/Game/LOGIC/DTO/ST_Info` Info))
  (set `self.Name` _name)
  (set `self.Description` _description)
  (set `self.Icon` _icon))