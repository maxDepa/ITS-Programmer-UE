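; BP_Chest is an interactable loot chest that rolls a random reward when used and can be opened only once.
; It compares one random roll against each LootsRewards entry's percentage in order and takes the first match.
; The reward type selects an item, experience, coin or HP handler, each currently only printing its value.
; All branches merge to set AlreadyOpened, which disables IsInteractable, and end the loop.
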(event `/Game/LOGIC/Model/Interface/BPI_Interactable.Interact`
  (`self.RollReward`))

(fn `GetCoin`
  (`KismetSystemLibrary.PrintString` (`KismetStringLibrary.Conv_IntToString` (`self.Coin`))))

(fn `GetExp`
  (`KismetSystemLibrary.PrintString` (`KismetStringLibrary.Conv_IntToString` (`self.Exp`))))

(fn `GetHp`
  (`KismetSystemLibrary.PrintString` (`KismetStringLibrary.Conv_IntToString` (`self.Hp`))))

(fn `GetItem`
  (`KismetSystemLibrary.PrintString` (`KismetSystemLibrary.GetObjectName` (`self.Item`))))

(fn `IsInteractable`
  (returns (IsInteractable :type Boolean))
  (return (not (`self.AlreadyOpened`))))

(fn `RollReward`
  (locals (RolledPercentage :type "Float (double-precision)" :default 0.0))
  (bind _output_get (set `local.RolledPercentage` (`KismetMathLibrary.RandomFloatInRange` 0.0 1.0)))
  (for _array_element (`self.LootsRewards`)
    (if (<= _output_get (`.Percentage_5_6CED94DA46C84C5061C689BF3ED7438F` (break `/Game/LOGIC/DTO/ST_LootReward` _array_element)))
      (switch `/Game/LOGIC/Common/ENUM_LootType` (break `/Game/LOGIC/DTO/ST_LootReward` _array_element)
        (:`NewEnumerator0`
          (`self.GetItem`))
        (:`NewEnumerator1`
          (`self.GetExp`))
        (:`NewEnumerator2`
          (`self.GetCoin`))
        (:`NewEnumerator3`
          (`self.GetHp`)))
      (set `self.AlreadyOpened` true)
      (break))))

(fn `UserConstructionScript`)